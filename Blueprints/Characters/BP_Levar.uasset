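; BP_Levar is the dialogue NPC Levar, whose Articy conversations can send the player to the Arena or ExplorablePrison levels.
; On interact, it starts a dialogue through the LoTE player controller, branching on the GameInstance first-dialogue flag and whether Levar is tired of talking.
; CheckDialogueLine tests specific lines in a chain of LevarChecksLine calls to set the entering level or update those flags.
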(event `self.ReceiveBeginPlay`
  (`parent.ReceiveBeginPlay`)
  (bind _asbp_lo_teplayer_controller (cast `/Game/LOTE/Blueprints/BP_LoTEPlayerController` (`GameplayStatics.GetPlayerController` 0)))
  (set `self.As BP Lo TEPlayer Controller_0` _asbp_lo_teplayer_controller))

(event `InteractableInterface.OnInteract`
  (bind _asbp_game_instance (cast `/Game/LOTE/Blueprints/BP_GameInstance` (`GameplayStatics.GetGameInstance`)))
  (set `self.As BP Game Instance` _asbp_game_instance)
  (if (`/Game/LOTE/Blueprints/BP_GameInstance.LevarFirstDialogue` _asbp_game_instance)
    (if (`self.LevarIsTiredOfTalking`)
      (`/Game/LOTE/Blueprints/BP_LoTEPlayerController.StartDialog` (stale `self.ReceiveBeginPlay` _asbp_lo_teplayer_controller) (`ArticyFunctionLibrary.ArticyId_GetObject` (struct :`Low` 1351 :`High` 16777216) null (`Lote_OmateDatabase.Get`)) self)
      (else
        (`/Game/LOTE/Blueprints/BP_LoTEPlayerController.StartDialog` (stale `self.ReceiveBeginPlay` _asbp_lo_teplayer_controller) (`ArticyFunctionLibrary.ArticyId_GetObject` (struct :`Low` 903 :`High` 16777216) null (`Lote_OmateDatabase.Get`)) self)))
    (else
      (`/Game/LOTE/Blueprints/BP_LoTEPlayerController.StartDialog` (`self.As BP Lo TEPlayer Controller_0`) (`ArticyFunctionLibrary.ArticyId_GetObject` (struct :`Low` 1377 :`High` 16777216) null (`Lote_OmateDatabase.Get`)) self))))

(event `self.CheckDialogueLine`
  (bind _isequal_ (`self.LevarChecksLine` (`ArticyFunctionLibrary.ArticyId_GetObject` (struct :`Low` 2663 :`High` 16777216) null (`Lote_OmateDatabase.Get`))))
  (if _isequal_
    (`/Game/LOTE/Blueprints/BP_LoTEPlayerController.Set Entering Level` (`self.As BP Lo TEPlayer Controller_0`) "Arena")
    (else
      (bind _isequal__2 (`self.LevarChecksLine` (`ArticyFunctionLibrary.ArticyId_GetObject` (struct :`Low` 2641 :`High` 16777216) null (`Lote_OmateDatabase.Get`))))
      (if _isequal__2
        (set `/Game/LOTE/Blueprints/BP_GameInstance.LevarFirstDialogue` false (`self.As BP Game Instance`))
        (`/Game/LOTE/Blueprints/BP_LoTEPlayerController.Set Entering Level` (`self.As BP Lo TEPlayer Controller_0`) "ExplorablePrison")
        (else
          (bind _isequal__3 (`self.LevarChecksLine` (`ArticyFunctionLibrary.ArticyId_GetObject` (struct :`Low` 2627 :`High` 16777216) null (`Lote_OmateDatabase.Get`))))
          (if _isequal__3
            (set `self.LevarIsTiredOfTalking` true :!label _label)
            (`KismetSystemLibrary.PrintString` "Hello" :!label _label_2)
            (else
              (bind _isequal__4 (`self.LevarChecksLine` (`ArticyFunctionLibrary.ArticyId_GetObject` (struct :`Low` 1079 :`High` 16777216) null (`Lote_OmateDatabase.Get`))))
              (if _isequal__4
                (goto _label)
                (else
                  (bind _isequal__5 (`self.LevarChecksLine` (`ArticyFunctionLibrary.ArticyId_GetObject` (struct :`Low` 1021 :`High` 16777216) null (`Lote_OmateDatabase.Get`))))
                  (if _isequal__5
                    (goto _label_2)))))))))))

(fn `UserConstructionScript`
  (`parent.UserConstructionScript`))