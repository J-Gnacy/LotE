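; Adalren is a character Blueprint for a friendly dialogue NPC who becomes the one-HP opponent in the tutorial fight.
; AdalrenDialogue starts an Articy conversation, and CheckDialogueLine turns Adalren hostile on a matching line, sets the player's enemy and begins combat.
; On death, combat ends, a knockdown animation plays and the actor is destroyed.
; LastBreathEvent then shows tutorial success if the player drank a potion or has full HP, otherwise failure.
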(event `self.ReceiveBeginPlay`
  (`parent.ReceiveBeginPlay`)
  (`self.SetCharacterName` "Adalren")
  (set `self.CurrentMood` "FRIENDLY")
  (bind _asbp_lo_teplayer_controller (cast `/Game/LOTE/Blueprints/BP_LoTEPlayerController` (`GameplayStatics.GetPlayerController` 0)))
  (set `self.As BP Lo TEPlayer Controller` _asbp_lo_teplayer_controller)
  (cast `/Game/LOTE/Blueprints/Characters/BP_LoTECharacter` (`GameplayStatics.GetPlayerCharacter` 0))
  (`self.SetCurrentHP` 1))

(event `self.CharacterKilled`
  (bind _knockeddownanimation (`self.KnockeddownAnimation`))
  (`/Game/LOTE/Blueprints/BP_LoTEPlayerController.End Combat` (`self.As BP Lo TEPlayer Controller`))
  (`SkeletalMeshComponent.PlayAnimation` (`self.Mesh`) _knockeddownanimation false)
  (bind _returnvalue (`AnimSequenceBase.GetPlayLength` _knockeddownanimation))
  (`KismetSystemLibrary.Delay` _returnvalue)
  (`self.K2_DestroyActor`)
  (`self.LastBreathEvent`))

(event `self.CheckDialogueLine`
  (bind _as_bp_lo_teplayer_controller (`self.As BP Lo TEPlayer Controller`))
  (bind _isequal_ (`/Game/LOTE/Blueprints/LoTEBlueprintFunctionLibrary.Check if Line Equals` (`ArticyFunctionLibrary.ArticyId_GetObject` (struct :`Low` 2475 :`High` 16777216) null (`Lote_OmateDatabase.Get`)) self (`GameplayStatics.GetPlayerController` 0)))
  (if _isequal_
    (`KismetSystemLibrary.PrintString` "hostelo")
    (set `self.CurrentMood` "HOSTILE")
    (bind _asbp_lo_techaracter (cast `/Game/LOTE/Blueprints/Characters/BP_LoTECharacter` (`GameplayStatics.GetPlayerCharacter` 0)))
    (set `LoTECharacter.Enemy` self _asbp_lo_techaracter)
    (`/Game/LOTE/Blueprints/BP_LoTEPlayerController.BeginCombat` _as_bp_lo_teplayer_controller)
    (`/Game/LOTE/Blueprints/BP_LoTEPlayerController.RemoveDialogFromViewport` _as_bp_lo_teplayer_controller)))

(event `self.LastBreathEvent`
  (bind _as_bp_lo_teplayer_controller (`self.As BP Lo TEPlayer Controller`))
  (bind _asbp_lo_techaracter (cast `/Game/LOTE/Blueprints/Characters/BP_LoTECharacter` (`GameplayStatics.GetPlayerCharacter` 0)))
  (bind _returnvalue (`self.GetCurrentHP` _asbp_lo_techaracter))
  (bind _returnvalue_2 (`self.GetMaxHP` _asbp_lo_techaracter))
  (bind _asbp_game_instance (cast `/Game/LOTE/Blueprints/BP_GameInstance` (`GameplayStatics.GetGameInstance`)))
  (if (or (`/Game/LOTE/Blueprints/BP_GameInstance.PotionDrank` _asbp_game_instance) (== _returnvalue _returnvalue_2))
    (bind _returnvalue_3 (`|CreateWidget` "/Game/LOTE/Blueprints/UI/TutorialSuccedeed.TutorialSuccedeed_C" _as_bp_lo_teplayer_controller))
    (`UserWidget.AddToViewport` _returnvalue_3 0)
    (else
      (bind _returnvalue_4 (`|CreateWidget` "/Game/LOTE/Blueprints/UI/TutorialFailed.TutorialFailed_C" _as_bp_lo_teplayer_controller))
      (`UserWidget.AddToViewport` _returnvalue_4 0))))

(fn `AdalrenDialogue`
  (params (Target :type "/Game/LOTE/Blueprints/BP_LoTEPlayerController Object Reference"))
  (`/Game/LOTE/Blueprints/BP_LoTEPlayerController.StartDialog` Target (`ArticyFunctionLibrary.ArticyId_GetObject` (struct :`Low` 2447 :`High` 16777216) null (`Lote_OmateDatabase.Get`)) self))

(fn `UserConstructionScript`
  (`parent.UserConstructionScript`))