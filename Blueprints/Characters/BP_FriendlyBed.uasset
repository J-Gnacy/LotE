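; BP_FriendlyBed is an interactable talking bed character that serves as a dialogue-driven way into the Arena level.
; On interact it starts a dialog on the LoTE player controller with an Articy line, naming itself as speaker.
; Its dialogue-line check compares against a specific Articy line and, on a match, sets the controller's entering level to Arena.
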(event `InteractableInterface.OnInteract`
  (`/Game/LOTE/Blueprints/BP_LoTEPlayerController.StartDialog` (`self.As BP Lo TEPlayer Controller`) (`ArticyFunctionLibrary.ArticyId_GetObject` (struct :`Low` 2382 :`High` 16777216) null (`Lote_OmateDatabase.Get`)) self))

(event `self.CheckDialogueLine`
  (bind _isequal_ (`/Game/LOTE/Blueprints/LoTEBlueprintFunctionLibrary.Check if Line Equals` (`ArticyFunctionLibrary.ArticyId_GetObject` (struct :`Low` 2649 :`High` 16777216) null (`Lote_OmateDatabase.Get`)) self (`self.As BP Lo TEPlayer Controller`)))
  (if _isequal_
    (`/Game/LOTE/Blueprints/BP_LoTEPlayerController.Set Entering Level` (`self.As BP Lo TEPlayer Controller`) "Arena")))

(fn `UserConstructionScript`
  (`parent.UserConstructionScript`))