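; BP_Cook is the cook character, an interactable NPC that opens a conversation with the player.
; On interaction it resolves an Articy ID to its dialogue object and passes it as the first line to StartDialog on the LoTE player controller, with itself as the speaker.
; It has no other active logic, as BeginPlay, overlap and Tick are disabled stubs.
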(event `InteractableInterface.OnInteract`
  (`/Game/LOTE/Blueprints/BP_LoTEPlayerController.StartDialog` (`self.As BP Lo TEPlayer Controller`) (`ArticyFunctionLibrary.ArticyId_GetObject` (struct :`Low` 1450 :`High` 16777216) null (`Lote_OmateDatabase.Get`)) self))

(fn `UserConstructionScript`
  (`parent.UserConstructionScript`))