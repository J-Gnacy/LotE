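; Player character for LoTE's turn-based combat, handling character creation, starting gear, animations and initiative.
; Character sheet widget events add and equip data-table weapons and armor, while creation completion loads stats from files and builds chat and info widgets.
; DoYourTurn passes the turn to the player controller, focusing the combat widget unless the character is tripped.
; A Tick gate allows clamped camera-boom rotation while right mouse is held.
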(event `DefaultCaptainCreated`
  (bind _foundwidgets (`WidgetBlueprintLibrary.GetAllWidgetsOfClass` "/Game/LOTE/Blueprints/UI/CaptainCreator.CaptainCreator_C"))
  (add `/Game/LOTE/Blueprints/UI/CaptainCreator.Create Captain` (`|GetArrayItem` _foundwidgets) (delegate `CreateCaptain`)))

(event `CreateCaptain`
  (bind _asbp_lo_teplayer_controller (cast `/Game/LOTE/Blueprints/BP_LoTEPlayerController` (`GameplayStatics.GetPlayerController` 0)))
  (`WidgetBlueprintLibrary.SetInputMode_GameAndUIEx` _asbp_lo_teplayer_controller null))

(event `self.ReceiveBeginPlay`
  (`self.SetCharacterName` "Kapitan")
  (`self.AddStandardGear`)
  (`self.InitializeAnimations`)
  (`self.Refresh Equipment`)
  (`self.InitializeInitiative`)
  (set `self.attackRange` 1.0)
  (bind _asbp_lo_teplayer_controller (cast `/Game/LOTE/Blueprints/BP_LoTEPlayerController` (`GameplayStatics.GetPlayerController` 0)))
  (set `self.As BP Lo TEPlayer Controller` _asbp_lo_teplayer_controller))

(event `LamArmorAdded`
  (bind _returnvalue (`|GetDataTableRow` "/Game/LOTE/Tables/ArmorsTable.ArmorsTable" "LamellarArmor")
    (:`then`
      (`/Game/LOTE/Blueprints/Eq/InventoryComponent.Add To Inventory` :`self` (`self.InventoryComponent`) :`Armor` _returnvalue)
      (set `self.ArmorEquipped` _returnvalue))))

(event `MenuCreated`
  (`KismetSystemLibrary.PrintString` "kurwa")
  (bind _foundwidgets (`WidgetBlueprintLibrary.GetAllWidgetsOfClass` "/Game/LOTE/Blueprints/UI/MenuWidget.MenuWidget_C"))
  (add `/Game/LOTE/Blueprints/UI/MenuWidget.GoingCreative` (`|GetArrayItem` _foundwidgets) (delegate `CreativeModeUsed`)))

(event `DaggerAdded`
  (bind _returnvalue (`|GetDataTableRow` "/Game/LOTE/Tables/WeaponsTable.WeaponsTable" "Dagger")
    (:`then`
      (`/Game/LOTE/Blueprints/Eq/InventoryComponent.AddWeapon` (`self.InventoryComponent`) _returnvalue)
      (set `self.WeaponEquipped` _returnvalue))))

(event `ShortswordAdded`
  (bind _returnvalue (`|GetDataTableRow` "/Game/LOTE/Tables/WeaponsTable.WeaponsTable" "Shortsword")
    (:`then`
      (`/Game/LOTE/Blueprints/Eq/InventoryComponent.AddWeapon` (`self.InventoryComponent`) _returnvalue)
      (set `self.WeaponEquipped` _returnvalue))))

(event `BattleaxeAdded`
  (bind _returnvalue (`|GetDataTableRow` "/Game/LOTE/Tables/WeaponsTable.WeaponsTable" "Battleaxe")
    (:`then`
      (`/Game/LOTE/Blueprints/Eq/InventoryComponent.AddWeapon` (`self.InventoryComponent`) _returnvalue)
      (set `self.WeaponEquipped` _returnvalue))))

(event `SwordAdded`
  (bind _returnvalue (`|GetDataTableRow` "/Game/LOTE/Tables/WeaponsTable.WeaponsTable" "Sword")
    (:`then`
      (`/Game/LOTE/Blueprints/Eq/InventoryComponent.AddWeapon` (`self.InventoryComponent`) _returnvalue)
      (set `self.WeaponEquipped` _returnvalue))))

(event `LongswordAdded`
  (bind _returnvalue (`|GetDataTableRow` "/Game/LOTE/Tables/WeaponsTable.WeaponsTable" "Longsword")
    (:`then`
      (`/Game/LOTE/Blueprints/Eq/InventoryComponent.AddWeapon` (`self.InventoryComponent`) _returnvalue)
      (set `self.WeaponEquipped` _returnvalue))))

(event `BFMaceAdded`
  (bind _returnvalue (`|GetDataTableRow` "/Game/LOTE/Tables/WeaponsTable.WeaponsTable" "BFMace")
    (:`then`
      (`/Game/LOTE/Blueprints/Eq/InventoryComponent.AddWeapon` (`self.InventoryComponent`) _returnvalue)
      (set `self.WeaponEquipped` _returnvalue))))

(event `BerdicheAdded`
  (bind _returnvalue (`|GetDataTableRow` "/Game/LOTE/Tables/WeaponsTable.WeaponsTable" "Berdiche")
    (:`then`
      (`/Game/LOTE/Blueprints/Eq/InventoryComponent.AddWeapon` (`self.InventoryComponent`) _returnvalue)
      (set `self.WeaponEquipped` _returnvalue))))

(event `GlaiveAdded`
  (bind _returnvalue (`|GetDataTableRow` "/Game/LOTE/Tables/WeaponsTable.WeaponsTable" "Glaive")
    (:`then`
      (`/Game/LOTE/Blueprints/Eq/InventoryComponent.AddWeapon` (`self.InventoryComponent`) _returnvalue)
      (set `self.WeaponEquipped` _returnvalue))))

(event `ThKnivesAdded`
  (bind _returnvalue (`|GetDataTableRow` "/Game/LOTE/Tables/WeaponsTable.WeaponsTable" "ThrowingKnife")
    (:`then`
      (`/Game/LOTE/Blueprints/Eq/InventoryComponent.AddWeapon` (`self.InventoryComponent`) _returnvalue)
      (set `self.WeaponEquipped` _returnvalue))))

(event `ShieldAdded`
  (bind _returnvalue (`|GetDataTableRow` "/Game/LOTE/Tables/WeaponsTable.WeaponsTable" "Shield")
    (:`then`
      (`/Game/LOTE/Blueprints/Eq/InventoryComponent.AddWeapon` (`self.InventoryComponent`) _returnvalue)
      (set `self.WeaponEquipped` _returnvalue))))

(event `CharacterSheetCreated`
  (bind _foundwidgets (`WidgetBlueprintLibrary.GetAllWidgetsOfClass` "/Game/LOTE/Blueprints/UI/CharacterSheet.CharacterSheet_C"))
  (bind _output (`|GetArrayItem` _foundwidgets))
  (add `/Game/LOTE/Blueprints/UI/CharacterSheet.Create Character` _output (delegate `CharacterCreated`))
  (`WidgetBlueprintLibrary.SetInputMode_GameAndUIEx` (`self.As BP Lo TEPlayer Controller`) null)
  (add `/Game/LOTE/Blueprints/UI/CharacterSheet.Get LeatherArmor` _output (delegate `LeatherArmorAdded`))
  (add `/Game/LOTE/Blueprints/UI/CharacterSheet.Get Lammelar Armor` _output (delegate `LamArmorAdded`))
  (add `/Game/LOTE/Blueprints/UI/CharacterSheet.Get Chainmail` _output (delegate `ChainmailAdded`))
  (add `/Game/LOTE/Blueprints/UI/CharacterSheet.GetDagger` _output (delegate `DaggerAdded`))
  (add `/Game/LOTE/Blueprints/UI/CharacterSheet.GetShortsword` _output (delegate `ShortswordAdded`))
  (add `/Game/LOTE/Blueprints/UI/CharacterSheet.GetBattleaxe` _output (delegate `BattleaxeAdded`))
  (add `/Game/LOTE/Blueprints/UI/CharacterSheet.GetSword` _output (delegate `SwordAdded`))
  (add `/Game/LOTE/Blueprints/UI/CharacterSheet.GetLongsword` _output (delegate `LongswordAdded`))
  (add `/Game/LOTE/Blueprints/UI/CharacterSheet.GetBFMace` _output (delegate `BFMaceAdded`))
  (add `/Game/LOTE/Blueprints/UI/CharacterSheet.GetBerdiche` _output (delegate `BerdicheAdded`))
  (add `/Game/LOTE/Blueprints/UI/CharacterSheet.GetGlaive` _output (delegate `GlaiveAdded`))
  (add `/Game/LOTE/Blueprints/UI/CharacterSheet.GetThKnives` _output (delegate `ThKnivesAdded`))
  (add `/Game/LOTE/Blueprints/UI/CharacterSheet.GetShield` _output (delegate `ShieldAdded`)))

(event `CreativeModeUsed`
  (`KismetSystemLibrary.PrintString` "niejebło"))

(event `LeatherArmorAdded`
  (bind _returnvalue (`|GetDataTableRow` "/Game/LOTE/Tables/ArmorsTable.ArmorsTable" "LeatherArmor")
    (:`then`
      (`/Game/LOTE/Blueprints/Eq/InventoryComponent.Add To Inventory` :`self` (`self.InventoryComponent`) :`Armor` _returnvalue)
      (set `self.ArmorEquipped` _returnvalue))))

(event `ChainmailAdded`
  (bind _returnvalue (`|GetDataTableRow` "/Game/LOTE/Tables/ArmorsTable.ArmorsTable" "Chainmail")
    (:`then`
      (`/Game/LOTE/Blueprints/Eq/InventoryComponent.Add To Inventory` :`self` (`self.InventoryComponent`) :`Armor` _returnvalue)
      (set `self.ArmorEquipped` _returnvalue))))

(event `CharacterCreated`
  (bind _returnvalue (`KismetSystemLibrary.GetProjectContentDirectory`))
  (`KismetSystemLibrary.PrintString` "There yet" true true (struct :`G` 0.66 :`B` 1.0 :`A` 1.0) 15.0)
  (`self.InitializeInitiative`)
  (`self.CreateChatWidget`)
  (`self.CreateInfoWidget`)
  (`self.StatsIntoArrayAlphabetically`)
  (bind _returnvalue_2 (`CharacterSheetLibrary.LoadFileToString` "zbiorczy" _returnvalue))
  (bind _returnvalue_3 (`CharacterSheetLibrary.LoadFileToStringArray` _returnvalue_2 _returnvalue))
  (`self.InitializeStats` _returnvalue_3)
  (bind _returnvalue_4 (`self.GetStrength`))
  (bind _returnvalue_5 (`self.GetDexterity`))
  (bind _returnvalue_6 (`self.GetSpeed`))
  (bind _returnvalue_7 (`self.GetEndurance`))
  (bind _returnvalue_8 (`self.GetSmarts`))
  (bind _returnvalue_9 (`self.GetPsyche`))
  (bind _returnvalue_10 (`self.GetSenses`))
  (`self.SetStats` _returnvalue_4 _returnvalue_5 _returnvalue_6 _returnvalue_7 _returnvalue_8 _returnvalue_9 _returnvalue_10)
  (`self.RefreshStats`)
  (bind _returnvalue_11 (`self.GetResistance`))
  (`self.SetDmgNegation` (+ _returnvalue_11 0))
  (bind _asbp_lo_teplayer_controller (cast `/Game/LOTE/Blueprints/BP_LoTEPlayerController` (`GameplayStatics.GetPlayerController` 0)))
  (add `/Game/LOTE/Blueprints/BP_LoTEPlayerController.ShowHideTest` _asbp_lo_teplayer_controller (delegate `SHideTest`)))

(event `SHideTest`
  (`/Engine/EditorBlueprintResources/StandardMacros.FlipFlop`
    (:`A`
      (bind _returnvalue (`|GenericCreateObject` "/Game/LOTE/Blueprints/UI/RollSheet.RollSheet_C" (`GameplayStatics.GetPlayerController` 0)))
      (bind _output_get (set `self.SHideVar` _returnvalue))
      (`UserWidget.AddToViewport` _output_get 0))
    (:`B`
      (`Widget.RemoveFromParent` _output_get))))

(event `self.ReceiveTick`
  (params (DeltaSeconds :type "Float (single-precision)"))
  (`|ExecutionSequence`
    (:`then_1`
      (`/Engine/EditorBlueprintResources/StandardMacros.Gate` true :!label _label
        (:`Exit`
          (if (`self.IsCameraMovable`)
            (`self.Camera Movement`)))))))

(event `Key|RightMouseButton`
  (params (Key :type "Key Structure"))
  (:`Pressed`
    (goto _label :!via `Open`))
  (:`Released`
    (goto _label :!via `Close`)))

(event `self.DoYourTurn`
  (`KismetSystemLibrary.PrintString` "Hello PC")
  (bind _asbp_lo_teplayer_controller (cast `/Game/LOTE/Blueprints/BP_LoTEPlayerController` (`GameplayStatics.GetPlayerController` 0)))
  (set `/Game/LOTE/Blueprints/BP_LoTEPlayerController.PlayersTurn` true _asbp_lo_teplayer_controller)
  (`Widget.RemoveFromParent` (`/Game/LOTE/Blueprints/BP_LoTEPlayerController.CombatPause` _asbp_lo_teplayer_controller))
  (if (!= (`self.isTripped`) true)
    (bind _combatwidget (`/Game/LOTE/Blueprints/BP_LoTEPlayerController.CombatWidget` _asbp_lo_teplayer_controller))
    (`/Game/LOTE/Blueprints/BP_LoTEPlayerController.LockOnWidget` _asbp_lo_teplayer_controller _asbp_lo_teplayer_controller _combatwidget _combatwidget)
    (if (and (< (`self.currentActions`) 1) (< (`self.currentPurchasableActions`) 1))
      _)
    (else
      (`/Game/LOTE/Blueprints/BP_LoTEPlayerController.DefensiveResourceManagement` _asbp_lo_teplayer_controller self)
      (`/Game/LOTE/Blueprints/BP_LoTEPlayerController.PlayIdleAnimation` _asbp_lo_teplayer_controller self))))

(fn `AddArmorToInventory`
  (params (Armor :type "/Game/LOTE/Tables/ArmorsStruct Structure"))
  (`/Game/LOTE/Blueprints/Eq/InventoryComponent.Add To Inventory` :`self` (`self.InventoryComponent`) :`Armor` Armor))

(fn `AddStandardGear`
  (bind _returnvalue (`|GetDataTableRow` "/Game/LOTE/Tables/WeaponsTable.WeaponsTable" "Fist")
    (:`then`
      (`/Game/LOTE/Blueprints/Eq/InventoryComponent.AddWeapon` (`self.InventoryComponent`) _returnvalue)
      (bind _returnvalue_2 (`|GetDataTableRow` "/Game/LOTE/Tables/ArmorsTable.ArmorsTable" "Naked")
        (:`then`
          (`/Game/LOTE/Blueprints/Eq/InventoryComponent.Add To Inventory` :`self` (`self.InventoryComponent`) :`Armor` _returnvalue_2))))))

(fn `AddWeaponToInventory`
  (params (Weapon :type "/Game/LOTE/Tables/WeaponsStruct Structure"))
  (`/Game/LOTE/Blueprints/Eq/InventoryComponent.AddWeapon` (`self.InventoryComponent`) Weapon))

(fn `Camera Movement`
  (bind _mousesensitivity (`self.MouseSensitivity`))
  (`SceneComponent.K2_SetWorldRotation` (`self.CameraBoom`) (`KismetMathLibrary.MakeRotator` (.roll (`SceneComponent.K2_GetComponentRotation` (`self.CameraBoom`))) (`KismetMathLibrary.FClamp` (+ (.pitch (`SceneComponent.K2_GetComponentRotation` (`self.CameraBoom`))) (* (`self.GetInputAxisKeyValue`) _mousesensitivity)) (`self.MinCameraClampValue`) (`self.MaxCameraClampValue`)) (+ (.yaw (`SceneComponent.K2_GetComponentRotation` (`self.CameraBoom`))) (* (`self.GetInputAxisKeyValue`) _mousesensitivity))) false false))

(fn `CreateChatWidget`
  (bind _asbp_lo_teplayer_controller (cast `/Game/LOTE/Blueprints/BP_LoTEPlayerController` (`GameplayStatics.GetPlayerController` 0)))
  (`/Game/LOTE/Blueprints/BP_LoTEPlayerController.CreateChatWidget` _asbp_lo_teplayer_controller))

(fn `CreateInfoWidget`
  (bind _asbp_lo_teplayer_controller (cast `/Game/LOTE/Blueprints/BP_LoTEPlayerController` (`GameplayStatics.GetPlayerController` 0)))
  (bind _returnvalue (`|CreateWidget` "/Game/LOTE/Blueprints/UI/InfoWidget.InfoWidget_C" _asbp_lo_teplayer_controller))
  (`UserWidget.AddToViewport` _returnvalue 0))

(fn `EquipCharacter`
  (params (Weapon :type "/Game/LOTE/Tables/WeaponsStruct Structure") (Armor :type "/Game/LOTE/Tables/ArmorsStruct Structure"))
  (`self.UseAddedWeapon` Weapon)
  (`self.UseAddedArmor` Armor)
  (`self.Refresh Equipment`))

(fn `InitializeAnimations`
  (set `self.AttackAnimation` "/Game/LOTE/Animations/Brawling/Prod/BrawlingComposite.BrawlingComposite")
  (set `self.CombatIdleAnimation` "/Game/LOTE/Animations/Brawling/Prod/BrawlingIdle.BrawlingIdle")
  (set `self.GetHitAnimation` "/Game/Steel_HitReact_Cringe_B.Steel_HitReact_Cringe_B")
  (set `self.LyingAnimation` "/Game/LOTE/Animations/2H/Old/Kek.Kek")
  (set `self.PushedAnimation` "/Game/LOTE/Animations/Maneuvers/KnockBack.KnockBack")
  (set `self.KnockeddownAnimation` "/Game/GetKnockedDown.GetKnockedDown")
  (set `self.BullrushAnimation` "/Game/LOTE/Animations/Maneuvers/Bullrush_2.Bullrush_2")
  (set `self.CatchAnimation` "/Game/LOTE/Animations/Maneuvers/Grab.Grab")
  (set `self.DodgeAnimation` "/Game/LOTE/Animations/Maneuvers/Dodge.Dodge")
  (set `self.TripAnimation` "/Game/LOTE/Animations/Maneuvers/Trip_2.Trip_2")
  (set `self.DeathAnimation` "/Game/LOTE/Animations/Steel_Death_B.Steel_Death_B"))

(fn `InitializeHUD`
  (`self.CreateChatWidget`)
  (`self.CreateInfoWidget`))

(fn `InitializeInitiative`
  (bind _returnvalue (`self.GetComponentByClass` "/Script/LoTE.InitiativeComponent"))
  (set `InitiativeComponent.initiative` 0 _returnvalue)
  (set `InitiativeComponent.initiativeBonus` 0 _returnvalue)
  (set `InitiativeComponent.hasRound` true _returnvalue)
  (set `InitiativeComponent.initiativeCounter` 0 _returnvalue))

(fn `Refresh Equipment`
  (bind _asbp_lo_teplayer_controller (cast `/Game/LOTE/Blueprints/BP_LoTEPlayerController` (`GameplayStatics.GetPlayerController` 0)))
  (`/Game/LOTE/Blueprints/BP_LoTEPlayerController.ShowHideInventory` _asbp_lo_teplayer_controller)
  (`/Game/LOTE/Blueprints/BP_LoTEPlayerController.ShowHideInventory` _asbp_lo_teplayer_controller))

(fn `UseAddedArmor`
  (params (Armor :type "/Game/LOTE/Tables/ArmorsStruct Structure"))
  (`self.AddArmorToInventory` Armor)
  (set `self.ArmorEquipped` Armor))

(fn `UseAddedWeapon`
  (params (Weapon :type "/Game/LOTE/Tables/WeaponsStruct Structure"))
  (`self.AddWeaponToInventory` Weapon)
  (set `self.WeaponEquipped` Weapon))

(fn `UserConstructionScript`)