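; BP_Garry is the NPC Garry, who starts friendly with 1 HP and opens Articy-driven dialogue when interacted with or forced.
; A check for a specific dialogue line turns him hostile, sets him as the player's enemy, begins combat through the player controller and closes the dialogue.
; His death ends combat, plays a knockdown animation, destroys him, flags GarryKilled on the game instance and loads CaptainsCell.
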(event `self.ReceiveBeginPlay`
  (`parent.ReceiveBeginPlay`)
  (`KismetSystemLibrary.PrintString` (`KismetSystemLibrary.GetDisplayName` self))
  (`self.SetCharacterName` "Garry")
  (set `self.CurrentMood` "FRIENDLY")
  (bind _asbp_lo_teplayer_controller (cast `/Game/LOTE/Blueprints/BP_LoTEPlayerController` (`GameplayStatics.GetPlayerController` 0)))
  (cast `/Game/LOTE/Blueprints/Characters/BP_LoTECharacter` (`GameplayStatics.GetPlayerCharacter` 0))
  (`self.SetCurrentHP` 1))

(event `InteractableInterface.OnInteract`
  (if (`|EnumEquality` (`self.CurrentMood`) "FRIENDLY")
    (`self.GarrysDialogue` (stale `self.ReceiveBeginPlay` _asbp_lo_teplayer_controller) self)))

(event `self.ForceDialogue`
  (`self.GarrysDialogue` (stale `self.ReceiveBeginPlay` _asbp_lo_teplayer_controller) self))

(event `self.CheckDialogueLine`
  (bind _isequal_ (`/Game/LOTE/Blueprints/LoTEBlueprintFunctionLibrary.Check if Line Equals` (`ArticyFunctionLibrary.ArticyId_GetObject` (struct :`Low` 387 :`High` 16777216) null (`Lote_OmateDatabase.Get`)) self (`GameplayStatics.GetPlayerController` 0)))
  (if _isequal_
    (`KismetSystemLibrary.PrintString` "hostelo")
    (set `self.CurrentMood` "HOSTILE")
    (bind _asbp_lo_techaracter (cast `/Game/LOTE/Blueprints/Characters/BP_LoTECharacter` (`GameplayStatics.GetPlayerCharacter` 0)))
    (set `LoTECharacter.Enemy` self _asbp_lo_techaracter)
    (`/Game/LOTE/Blueprints/BP_LoTEPlayerController.BeginCombat` (stale `self.ReceiveBeginPlay` _asbp_lo_teplayer_controller))
    (`/Game/LOTE/Blueprints/BP_LoTEPlayerController.RemoveDialogFromViewport` (stale `self.ReceiveBeginPlay` _asbp_lo_teplayer_controller))))

(event `self.CharacterKilled`
  (bind _knockeddownanimation (`self.KnockeddownAnimation`))
  (`/Game/LOTE/Blueprints/BP_LoTEPlayerController.End Combat` (stale `self.ReceiveBeginPlay` _asbp_lo_teplayer_controller))
  (`SkeletalMeshComponent.PlayAnimation` (`self.Mesh`) _knockeddownanimation false)
  (bind _returnvalue (`AnimSequenceBase.GetPlayLength` _knockeddownanimation))
  (`KismetSystemLibrary.Delay` _returnvalue)
  (`self.K2_DestroyActor`)
  (`self.LastBreathEvent`))

(event `self.LastBreathEvent`
  (bind _asbp_game_instance (cast `/Game/LOTE/Blueprints/BP_GameInstance` (`GameplayStatics.GetGameInstance`))
    (:`then`
      (set `/Game/LOTE/Blueprints/BP_GameInstance.GarryKilled` true _asbp_game_instance)
      (`GameplayStatics.OpenLevel` "CaptainsCell"))
    (:`CastFailed`
      (`KismetSystemLibrary.PrintString` "Cast failed"))))

(fn `GarrysDialogue`
  (params (self2 :type "/Game/LOTE/Blueprints/BP_LoTEPlayerController Object Reference") (SpeakerCharacter :type "MonsterCharacter Object Reference"))
  (`/Game/LOTE/Blueprints/BP_LoTEPlayerController.StartDialog` self2 (`ArticyFunctionLibrary.ArticyId_GetObject` (struct :`Low` 335 :`High` 16777216) null (`Lote_OmateDatabase.Get`)) SpeakerCharacter))

(fn `UserConstructionScript`
  (`parent.UserConstructionScript`))