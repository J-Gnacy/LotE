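; BP_Daren is an NPC character that starts an Articy-driven dialogue when the player interacts with it.
; It caches the LoTE player controller on BeginPlay and, on interact, asks it to start dialogue from an Articy object with itself as speaker.
; A helper function checks whether a given line equals one for this speaker, while the CheckDialogueLine event is left empty.
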(event `self.ReceiveBeginPlay`
  (`parent.ReceiveBeginPlay`)
  (bind _asbp_lo_teplayer_controller (cast `/Game/LOTE/Blueprints/BP_LoTEPlayerController` (`GameplayStatics.GetPlayerController` 0)))
  (set `self.As BP Lo TEPlayer Controller_0` _asbp_lo_teplayer_controller))

(event `InteractableInterface.OnInteract`
  (`/Game/LOTE/Blueprints/BP_LoTEPlayerController.StartDialog` (`self.As BP Lo TEPlayer Controller_0`) (`ArticyFunctionLibrary.ArticyId_GetObject` (struct :`Low` 1096 :`High` 16777216) null (`Lote_OmateDatabase.Get`)) self))

(event `self.CheckDialogueLine`)

(fn `UserConstructionScript`
  (`parent.UserConstructionScript`))