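; BP_Marcus is an interactable character whose Articy dialogue tracks the outcome of a potion event.
; OnInteract starts dialogue through the player controller, branching on PotionSpilt to choose the first line.
; CheckDialogueLine uses the MarcusChecksLine helper to match specific lines, setting PotionDrank on BP_GameInstance or the local PotionSpilt flag that feeds later interactions.
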(event `InteractableInterface.OnInteract`
  (if (`self.PotionSpilt`)
    (`/Game/LOTE/Blueprints/BP_LoTEPlayerController.StartDialog` (`self.As BP Lo TEPlayer Controller`) (`ArticyFunctionLibrary.ArticyId_GetObject` (struct :`Low` 2270 :`High` 16777216) null (`Lote_OmateDatabase.Get`)) self)
    (else
      (`/Game/LOTE/Blueprints/BP_LoTEPlayerController.StartDialog` (`self.As BP Lo TEPlayer Controller`) (`ArticyFunctionLibrary.ArticyId_GetObject` (struct :`Low` 2081 :`High` 16777216) null (`Lote_OmateDatabase.Get`)) self))))

(event `self.CheckDialogueLine`
  (bind _isequal_ (`self.MarcusChecksLine` (`ArticyFunctionLibrary.ArticyId_GetObject` (struct :`Low` 2241 :`High` 16777216) null (`Lote_OmateDatabase.Get`))))
  (if _isequal_
    (bind _asbp_game_instance (cast `/Game/LOTE/Blueprints/BP_GameInstance` (`GameplayStatics.GetGameInstance`)))
    (set `/Game/LOTE/Blueprints/BP_GameInstance.PotionDrank` true _asbp_game_instance)
    (else
      (bind _isequal__2 (`self.MarcusChecksLine` (`ArticyFunctionLibrary.ArticyId_GetObject` (struct :`Low` 2263 :`High` 16777216) null (`Lote_OmateDatabase.Get`))))
      (if _isequal__2
        (set `self.PotionSpilt` true)))))

(fn `UserConstructionScript`
  (`parent.UserConstructionScript`))