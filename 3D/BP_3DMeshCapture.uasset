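; 3D mesh capture actor whose skeletal mesh mirrors the armor equipped by the player character.
; On BeginPlay it refreshes the mesh, then binds the same update to the LoTE player controller's armor-change event.
; Each update copies the mesh from the character's ArmorEquipped and reinitializes the pose, so no Tick polling is used.
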(event `self.ReceiveBeginPlay`
  (`self.UpdateMesh`)
  (bind _asbp_lo_teplayer_controller (cast `/Game/LOTE/Blueprints/BP_LoTEPlayerController` (`GameplayStatics.GetPlayerController` 0)))
  (add `/Game/LOTE/Blueprints/BP_LoTEPlayerController.ChangeArmor` _asbp_lo_teplayer_controller (delegate `UpdateMesh`)))

(event `UpdateMesh`
  (bind _asbp_lo_techaracter (cast `/Game/LOTE/Blueprints/Characters/BP_LoTECharacter` (`GameplayStatics.GetPlayerCharacter` 0)))
  (bind (_armorequipped_name _armorequipped_protection _armorequipped_movepenalty _armorequipped_price _armorequipped_weight _armorequipped_thumbnail _armorequipped_mesh) (break `/Game/LOTE/Tables/ArmorsStruct` (`/Game/LOTE/Blueprints/Characters/BP_LoTECharacter.ArmorEquipped` _asbp_lo_techaracter)))
  (`SkinnedMeshComponent.SetSkinnedAssetAndUpdate` (`self.SkeletalMesh`) _armorequipped_mesh true))

(event `self.ReceiveTick`
  (params (DeltaSeconds :type "Float (single-precision)")))

(fn `UserConstructionScript`)